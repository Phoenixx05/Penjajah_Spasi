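; BP_BoosterHealth is a health pickup for BP_Pesawat, triggered when that actor overlaps its sphere.
; The Booster event hides the heart, adds health to the overlapping actor, then waits on a delay.
; If health is then at or below the 15000 threshold, it sets health to that value and destroys itself.
; Otherwise it repeats the add-and-wait loop, destroying itself once the counter reaches five.
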(event `self.Sphere.OnComponentBeginOverlap`
  (params (OverlappedComponent :type "PrimitiveComponent Object Reference") (OtherActor :type "Actor Object Reference") (OtherComp :type "PrimitiveComponent Object Reference") (OtherBodyIndex :type Integer) (bFromSweep :type Boolean) (SweepResult :type "HitResult Structure (by ref)"))
  (bind _asbp_pesawat (cast `/Game/Penjelajah_Spasi/Playable/BP_Pesawat` OtherActor))
  (set `self.Pesawat` _asbp_pesawat)
  (`self.Booster`))

(event `/Game/Penjelajah_Spasi/Booster/BP_BoosterInterface.Booster`
  (bind _pesawat (`self.Pesawat`))
  (`SceneComponent.SetHiddenInGame` (`self.Pickup_Heart`) true false)
  (set `/Game/Penjelajah_Spasi/Playable/BP_Pesawat.Health` (+ (`/Game/Penjelajah_Spasi/Playable/BP_Pesawat.Health` _pesawat) 100) _pesawat :!label _label)
  (`/Engine/EditorBlueprintResources/StandardMacros.IncrementInt` (`self.Counter`)
    (:`  `
      (`KismetSystemLibrary.Delay` 3.0)
      (if (>= 15000 (`/Game/Penjelajah_Spasi/Playable/BP_Pesawat.Health` (`self.Pesawat`)))
        (set `/Game/Penjelajah_Spasi/Playable/BP_Pesawat.Health` 15000 (`self.Pesawat`))
        (elif (== 5 (`self.Counter`))
          _
          (else
            (goto _label))))
      (`self.K2_DestroyActor`))))

(fn `UserConstructionScript`
  (`parent.UserConstructionScript`))