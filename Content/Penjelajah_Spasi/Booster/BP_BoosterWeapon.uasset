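; BP_BoosterWeapon is a weapon power-up pickup that temporarily switches the player ship's projectile to a blue laser.
; When BP_Pesawat overlaps its Sphere, it stores the ship, hides the Lightsaber component and sets the ship's Class variable to BP_BlueLaser.
; After a seven-second delay it resets that class to BP_Bullet and destroys itself.
; The Sphere's collision stays unchanged during the delay, and a debug "Hello" print remains.
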(event `self.Sphere.OnComponentBeginOverlap`
  (params (OverlappedComponent :type "PrimitiveComponent Object Reference") (OtherActor :type "Actor Object Reference") (OtherComp :type "PrimitiveComponent Object Reference") (OtherBodyIndex :type Integer) (bFromSweep :type Boolean) (SweepResult :type "HitResult Structure (by ref)"))
  (bind _asbp_pesawat (cast `/Game/Penjelajah_Spasi/Playable/BP_Pesawat` OtherActor))
  (set `self.Pesawat` _asbp_pesawat)
  (`self.Booster`))

(event `/Game/Penjelajah_Spasi/Booster/BP_BoosterInterface.Booster`
  (`KismetSystemLibrary.PrintString` "Hello")
  (`SceneComponent.SetHiddenInGame` (`self.lightsaber`) true false)
  (set `/Game/Penjelajah_Spasi/Playable/BP_Pesawat.Class` "/Game/Penjelajah_Spasi/Weapon/BP_BlueLaser.BP_BlueLaser_C" (`self.Pesawat`))
  (`KismetSystemLibrary.Delay` 7.0)
  (set `/Game/Penjelajah_Spasi/Playable/BP_Pesawat.Class` "/Game/Penjelajah_Spasi/Weapon/BP_Bullet.BP_Bullet_C" (`self.Pesawat`))
  (`self.K2_DestroyActor`))

(fn `UserConstructionScript`
  (`parent.UserConstructionScript`))