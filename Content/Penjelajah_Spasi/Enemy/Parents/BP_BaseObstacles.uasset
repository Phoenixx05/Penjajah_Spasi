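; BP_BaseObstacles is a parent Blueprint for obstacles that damage the player ship and can be shot for score.
; Capsule overlap with BP_Pesawat subtracts DMG from the ship's Health and destroys the obstacle.
; AnyDamage lowers HP and calls a score check, which adds Score to BP_GameIntance only when HP reaches zero or below.
; The obstacle is destroyed after any damage, even if HP remains.
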(event `self.ReceiveActorBeginOverlap`
  (params (OtherActor :type "Actor Object Reference")))

(event `self.Capsule.OnComponentBeginOverlap`
  (params (OverlappedComponent :type "PrimitiveComponent Object Reference") (OtherActor :type "Actor Object Reference") (OtherComp :type "PrimitiveComponent Object Reference") (OtherBodyIndex :type Integer) (bFromSweep :type Boolean) (SweepResult :type "HitResult Structure (by ref)"))
  ;[1 1 1] Damage ke Pesawat
  (bind _asbp_pesawat (cast `/Game/Penjelajah_Spasi/Playable/BP_Pesawat` OtherActor))
  (set `/Game/Penjelajah_Spasi/Playable/BP_Pesawat.Health` (- (`/Game/Penjelajah_Spasi/Playable/BP_Pesawat.Health` _asbp_pesawat) (`self.DMG`)) _asbp_pesawat)
  (`self.K2_DestroyActor`))

(event `self.ReceiveAnyDamage`
  (params (Damage :type "Float (single-precision)") (DamageType :type "DamageType Object Reference") (InstigatedBy :type "Controller Object Reference") (DamageCauser :type "Actor Object Reference"))
  ;[1 1 1] Damage ke Enemy
  (set `self.HP` (`KismetMathLibrary.FTrunc` (- (`self.HP`) Damage)))
  (`self.SetScore?`)
  (`self.K2_DestroyActor`))

(event `SetScore?`
  ;[0.9896 0.9792 1 1 50] SetScore?
  (if (<= (`self.HP`) 0)
    (bind _asbp_game_intance (cast `/Game/Penjelajah_Spasi/BP_GameIntance` (`GameplayStatics.GetGameInstance`)))
    (set `/Game/Penjelajah_Spasi/BP_GameIntance.Score` (+ (`/Game/Penjelajah_Spasi/BP_GameIntance.Score` _asbp_game_intance) (`self.Score`)) _asbp_game_intance)
    (`self.K2_DestroyActor`)))

(fn `UserConstructionScript`)