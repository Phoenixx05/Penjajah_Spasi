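; UFO boss that shows a health widget and begins attacking once Tick finds no BP_TeleportPoint in the level.
; Two looping delays drive attacks: red lasers from an arrow, and batches of random enemies inside BP_MapBoss's SpawnBox.
; Damage lowers Health, while DMG_RedLaser adds it back; death removes the widget, spawns a teleport point, and destroys spawned enemies and itself.
; The timeline movement logic is never executed.
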(event `DMG_RedLaser`
  (params (DMG :type "Float (double-precision)"))
  ;[1 1 1] Health
  (set `self.Health` (+ (`self.Health`) DMG)))

(event `self.ReceiveAnyDamage`
  (params (Damage :type "Float (single-precision)") (DamageType :type "DamageType Object Reference") (InstigatedBy :type "Controller Object Reference") (DamageCauser :type "Actor Object Reference"))
  ;[1 1 1] Health
  (set `self.Health` (- (`self.Health`) Damage))
  (if (<= (`self.Health`) 0.0)
    (`/Engine/EditorBlueprintResources/StandardMacros.DoOnce` false
      (:`Completed`
        (`Widget.RemoveFromParent` (`self.HealthUI`))
        (if (== (`self.SpawnTeleport?`) false)
          (`|SpawnActorFromClass` "/Game/Penjelajah_Spasi/Teleport/BP_TeleportPoint.BP_TeleportPoint_C" (`KismetMathLibrary.MakeTransform` (-15070.931099 -1741.280743 26739.018325) (struct :`Yaw` 90.0)) "Undefined" "MultiplyWithRoot" null null)
          (set `self.SpawnTeleport?` true)
          (for _array_element (`self.Enemies`)
            (`/Engine/EditorBlueprintResources/StandardMacros.IsValid` _array_element
              (:`Is Valid`
                (`self.K2_DestroyActor` _array_element))))
          (`GameplayStatics.PlaySoundAtLocation` "/Game/Penjelajah_Spasi/Sounds_Musics/boss_dead.boss_dead" (`SceneComponent.K2_GetComponentLocation` (`self.BossUfo`)) (struct) 1.0 1.0 0.0 null null null null)
          (`KismetSystemLibrary.Delay` 0.2)
          (`self.K2_DestroyActor`))))))

(event `self.ReceiveBeginPlay`
  ;[1 1 1] Widget Boss Health
  (bind _returnvalue (`|CreateWidget` "/Game/Penjelajah_Spasi/Enemy/Parents/Boss/WB_BossFightHealth.WB_BossFightHealth_C" null self))
  (`UserWidget.AddToViewport` _returnvalue 0)
  (set `self.HealthUI` _returnvalue))

(event `self.ReceiveTick`
  (params (DeltaSeconds :type "Float (single-precision)"))
  (bind _returnvalue (`GameplayStatics.GetActorOfClass` "/Game/Penjelajah_Spasi/Teleport/BP_TeleportPoint.BP_TeleportPoint_C"))
  (`/Engine/EditorBlueprintResources/StandardMacros.IsValid` _returnvalue
    (:`Is Not Valid`
      (`self.SetActorTickEnabled` false)
      (`/Game/Penjelajah_Spasi/Enemy/Parents/Boss/BPI_BossFight.Attack`))))

(event `Shoot`
  ;[1 1 1] Spawn Bullet - Nembak
  (`KismetSystemLibrary.PrintString` "Hello")
  (`GameplayStatics.PlaySoundAtLocation` "/Game/Penjelajah_Spasi/Sounds_Musics/boss_attack.boss_attack" (`SceneComponent.K2_GetComponentLocation` (`self.BossUfo`)) (struct) 1.0 1.0 0.0 null null null null)
  (`|SpawnActorFromClass` "/Game/Penjelajah_Spasi/Weapon/BP_RedLaser.BP_RedLaser_C" (`KismetMathLibrary.MakeTransform` (`SceneComponent.K2_GetComponentLocation` (`self.Arrow`))) "Undefined" "MultiplyWithRoot" null null))

(event `/Game/Penjelajah_Spasi/Enemy/Parents/Boss/BPI_BossFight.Attack`
  ;[1 1 1] Attack Boss
  (`|ExecutionSequence`
    (:`then_0`
      (`self.Shoot` :!label _label)
      (`KismetSystemLibrary.Delay` 1.0)
      (goto _label))
    (:`then_1`
      (`self.spawnObstacles` :!label _label_2)
      (`KismetSystemLibrary.Delay` 3.0)
      (goto _label_2))))

(event `spawnObstacles`
  ;[1 1 1] Spawn Enemies (Obstacles)
  (`GameplayStatics.PlaySoundAtLocation` "/Game/Penjelajah_Spasi/Sounds_Musics/spawn_obstacles_boss.spawn_obstacles_boss" (`SceneComponent.K2_GetComponentLocation` (`self.BossUfo`)) (struct) 1.0 1.0 0.0 null null null null)
  (bind _returnvalue (`GameplayStatics.GetActorOfClass` "/Game/Penjelajah_Spasi/Map/BP_MapBoss.BP_MapBoss_C"))
  (for _ (range 5)
    (bind _spawnbox (`/Game/Penjelajah_Spasi/Map/BP_MapBoss.SpawnBox` _returnvalue))
    (bind _returnvalue_2 (`|SpawnActorFromClass` (`KismetArrayLibrary.Array_Random` (`self.TipeMusuh`)) (`KismetMathLibrary.MakeTransform` (`KismetMathLibrary.RandomPointInBoundingBox` (`SceneComponent.K2_GetComponentLocation` _spawnbox) (`BoxComponent.BoxExtent` _spawnbox))) "Undefined" "MultiplyWithRoot" null null))
    (`KismetArrayLibrary.Array_Add` (`self.Enemies`) _returnvalue_2)))

(fn `UserConstructionScript`)