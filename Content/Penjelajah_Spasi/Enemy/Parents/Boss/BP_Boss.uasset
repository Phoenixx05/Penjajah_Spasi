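; BP_Boss is a boss enemy character, filed as a parent class, with health, a montage attack and an on-screen health bar.
; BeginPlay creates the WB_BossFightHealth widget, and Tick sets its bar from Health on a fixed 100-point scale.
; Attack plays a montage behind an IsAttacking guard that clears on completion.
; AnyDamage subtracts Health and, at zero or below, disables movement and ragdolls the mesh.
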(event `self.ReceiveBeginPlay`
  (bind _returnvalue (`|CreateWidget` "/Game/Penjelajah_Spasi/Enemy/Parents/Boss/WB_BossFightHealth.WB_BossFightHealth_C"))
  (`UserWidget.AddToViewport` _returnvalue 0)
  (set `self.healthUI` _returnvalue))

(event `self.ReceiveTick`
  (params (DeltaSeconds :type "Float (single-precision)"))
  (`ProgressBar.SetPercent` (`/Game/Penjelajah_Spasi/Enemy/Parents/Boss/WB_BossFightHealth.HealthBar` (`self.healthUI`)) (/ (`self.health`) 100.0)))

(event `/Game/Penjelajah_Spasi/Enemy/Parents/Boss/BPI_BossFight.Attack`
  ;[1 1 1] Attack
  (if (not (`self.isAttacking?`))
    (`|PlayMontage` (`self.Mesh`)
      (:`then`
        (`KismetSystemLibrary.PrintString` "ATTACK")
        (set `self.isAttacking?` true))
      (:`OnCompleted`
        (set `self.isAttacking?` false)))))

(event `self.ReceiveAnyDamage`
  (params (Damage :type "Float (single-precision)") (DamageType :type "DamageType Object Reference") (InstigatedBy :type "Controller Object Reference") (DamageCauser :type "Actor Object Reference"))
  ;[1 1 1] Health
  (set `self.health` (- (`self.health`) Damage))
  (`KismetSystemLibrary.PrintString` (`KismetStringLibrary.Conv_DoubleToString` (`self.health`)))
  (if (<= (`self.health`) 0.0)
    (`CharacterMovementComponent.DisableMovement` (`self.CharacterMovement`))
    (`PrimitiveComponent.SetSimulatePhysics` (`self.Mesh`) true)))

(fn `UserConstructionScript`)