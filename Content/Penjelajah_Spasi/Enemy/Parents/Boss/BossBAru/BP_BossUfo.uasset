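; BP_BossUfo is a UFO boss enemy that tracks its own health and shows a boss fight health bar.
; On BeginPlay it creates the WB_BossFightHealth widget with itself as owner, adds it to the viewport and stores it as HealthUI.
; AnyDamage subtracts damage from Health and prints the result; the zero-health check has no death logic yet, and nothing here updates the widget.
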(event `self.ReceiveAnyDamage`
  (params (Damage :type "Float (single-precision)") (DamageType :type "DamageType Object Reference") (InstigatedBy :type "Controller Object Reference") (DamageCauser :type "Actor Object Reference"))
  ;[1 1 1] Health
  (bind _output_get (set `self.health` (- (`self.health`) Damage)))
  (`KismetSystemLibrary.PrintString` (`KismetStringLibrary.Conv_DoubleToString` _output_get))
  (if (<= (`self.health`) 0.0)
    _))

(event `self.ReceiveBeginPlay`
  ;[1 1 1] Widget Boss Health
  (bind _returnvalue (`|CreateWidget` "/Game/Penjelajah_Spasi/Enemy/Parents/Boss/WB_BossFightHealth.WB_BossFightHealth_C" null self))
  (`UserWidget.AddToViewport` _returnvalue 0)
  (set `self.healthUI` _returnvalue))

(fn `UserConstructionScript`)