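; Endless map spawner for Penjelajah Spasi that keeps a rolling chain of BP_MapBase segments along X for the player's BP_Pesawat.
; BeginPlay spawns the initial segments and binds their Box overlaps.
; Each player overlap moves Cube to the oldest segment's Box1, appends a segment, then destroys the oldest with its enemies.
; Tick shifts Bulan (the moon) by the player's X travel, keeping its relative distance constant.
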(event `self.ReceiveBeginPlay`
  (bind _asbp_pesawat (cast `/Game/Penjelajah_Spasi/Playable/BP_Pesawat` (`GameplayStatics.GetPlayerPawn` 0)))
  (bind _output_get (set `self.As BP Pesawat` _asbp_pesawat))
  (bind _returnvalue_x (`KismetMathLibrary.BreakVector` (`self.K2_GetActorLocation` _output_get)))
  (set `self.SpawnPlayerX` _returnvalue_x)
  (set `self.MoonSpawn` (`SceneComponent.K2_GetComponentLocation` (`self.bulan`)))
  (set `self.LastLocation` (`SceneComponent.K2_GetComponentLocation` (`self.DefaultSceneRoot`)))
  (for _ (range 4)
    (bind _returnvalue (`|SpawnActorFromClass` "/Game/Penjelajah_Spasi/Map/BP_MapBase.BP_MapBase_C" (`KismetMathLibrary.MakeTransform` (`self.LastLocation`)) "Undefined" "MultiplyWithRoot" null null))
    (add `PrimitiveComponent.OnComponentBeginOverlap` (`/Game/Penjelajah_Spasi/Map/BP_MapBase.Box` _returnvalue) (delegate `Overlap`))
    (`KismetArrayLibrary.Array_Add` (`self.ChildActor`) _returnvalue)
    (set `self.LastLocation` (+ (`self.LastLocation`) (make `IntVector` (`self.SpaceBetweenMap`))))))

(event `Overlap`
  (params (OverlappedComponent :type "PrimitiveComponent Object Reference") (OtherActor :type "Actor Object Reference") (OtherComp :type "PrimitiveComponent Object Reference") (OtherBodyIndex :type Integer) (bFromSweep :type Boolean) (SweepResult :type "HitResult Structure (by ref)"))
  (bind _childactor (`self.ChildActor`))
  (bind _output (`|GetArrayItem` _childactor))
  (cast `/Game/Penjelajah_Spasi/Playable/BP_Pesawat` OtherActor)
  (`SceneComponent.K2_SetWorldLocation` (`self.Cube`) (`SceneComponent.K2_GetComponentLocation` (`/Game/Penjelajah_Spasi/Map/BP_MapBase.Box1` (`|GetArrayItem` (`self.ChildActor`)))) false false)
  (bind _returnvalue (`|SpawnActorFromClass` "/Game/Penjelajah_Spasi/Map/BP_MapBase.BP_MapBase_C" (`KismetMathLibrary.MakeTransform` (`self.LastLocation`)) "Undefined" "MultiplyWithRoot" null null))
  (add `PrimitiveComponent.OnComponentBeginOverlap` (`/Game/Penjelajah_Spasi/Map/BP_MapBase.Box` _returnvalue) (delegate `Overlap`))
  (`KismetArrayLibrary.Array_Add` (`self.ChildActor`) _returnvalue)
  (set `self.LastLocation` (+ (`self.LastLocation`) (make `IntVector` (`self.SpaceBetweenMap`))))
  (`/Engine/EditorBlueprintResources/StandardMacros.IsValid` _output
    (:`Is Valid`
      (for _array_element (`/Game/Penjelajah_Spasi/Map/BP_MapBase.Enemy` _output)
        (`/Engine/EditorBlueprintResources/StandardMacros.IsValid` _array_element
          (:`Is Valid`
            (`self.K2_DestroyActor` _array_element))))
      (`self.K2_DestroyActor` _output)
      (`KismetArrayLibrary.Array_Remove` _childactor))))

(event `self.ReceiveTick`
  (params (DeltaSeconds :type "Float (single-precision)"))
  (bind (_moonspawn_x _moonspawn_y _moonspawn_z) (`KismetMathLibrary.BreakVector` (`self.MoonSpawn`)))
  (bind _returnvalue_x (`KismetMathLibrary.BreakVector` (`self.K2_GetActorLocation` (`self.As BP Pesawat`))))
  (`SceneComponent.K2_SetWorldLocation` (`self.bulan`) (`KismetMathLibrary.MakeVector` (+ _moonspawn_x (- _returnvalue_x (`self.SpawnPlayerX`))) _moonspawn_y _moonspawn_z) false false))

(fn `Spawn`)

(fn `UserConstructionScript`)