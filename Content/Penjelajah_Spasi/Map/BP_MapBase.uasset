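; BP_MapBase is a map actor for Penjelajah_Spasi that fills its spawn volume with random obstacles and boosters.
; On BeginPlay, two fixed-count loops spawn many random classes from TipeMusuh and a few from TipeBooster.
; Each lands at a random point inside the SpawnLoc box and is stored in the Enemy or Booster array.
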(event `self.ReceiveBeginPlay`
  (bind _spawnloc (`self.SpawnLoc`))
  (bind _spawnloc_2 (`self.SpawnLoc`))
  ;[1 1 1] Spawn Obstacles
  (for _ (range 45)
    (bind _returnvalue (`|SpawnActorFromClass` (`KismetArrayLibrary.Array_Random` (`self.TipeMusuh`)) (`KismetMathLibrary.MakeTransform` (`KismetMathLibrary.RandomPointInBoundingBox` (`SceneComponent.K2_GetComponentLocation` _spawnloc_2) (`BoxComponent.BoxExtent` _spawnloc_2))) "Undefined" "MultiplyWithRoot" null null))
    (`KismetArrayLibrary.Array_Add` (`self.Enemy`) _returnvalue))
  ;[1 1 1] Spawn Booster
  (for _ (range 3)
    (bind _returnvalue_2 (`|SpawnActorFromClass` (`KismetArrayLibrary.Array_Random` (`self.TipeBooster`)) (`KismetMathLibrary.MakeTransform` (`KismetMathLibrary.RandomPointInBoundingBox` (`SceneComponent.K2_GetComponentLocation` _spawnloc) (`BoxComponent.BoxExtent` _spawnloc))) "Undefined" "MultiplyWithRoot" null null))
    (`KismetArrayLibrary.Array_Add` (`self.Booster`) _returnvalue_2)))

(fn `UserConstructionScript`)