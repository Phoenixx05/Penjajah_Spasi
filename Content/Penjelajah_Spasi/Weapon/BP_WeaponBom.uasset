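; Bomb weapon actor that explodes shortly after spawning and detects obstacles in its blast sphere.
; BeginPlay keeps Sphere collision off during a brief fuse, then enables it, plays explosion particles and sound, and hides the Bom component before a delayed self-destroy.
; Sphere overlaps with BP_BaseObstacles copy that obstacle's HP into DMG, matching damage to its health; no damage is applied here.
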(event `self.ReceiveBeginPlay`
  (`parent.ReceiveBeginPlay`)
  (`PrimitiveComponent.SetCollisionEnabled` (`self.Sphere`) "NoCollision")
  (`KismetSystemLibrary.Delay` 0.2)
  (`GameplayStatics.SpawnEmitterAtLocation` "/Game/StarterContent/Particles/P_Explosion.P_Explosion" (`self.K2_GetActorLocation`) (struct) (3.0 1.0 1.0))
  (`PrimitiveComponent.SetCollisionEnabled` (`self.Sphere`) "QueryAndPhysics")
  (`GameplayStatics.PlaySoundAtLocation` "/Game/StarterContent/Audio/Explosion_Cue.Explosion_Cue" (`self.K2_GetActorLocation`) (struct) 1.0 1.0 0.0 null null null null)
  (`SceneComponent.SetHiddenInGame` (`self.bom`) true false)
  (`KismetSystemLibrary.Delay` 2.0)
  (`self.K2_DestroyActor`))

(event `self.Sphere.OnComponentBeginOverlap`
  (params (OverlappedComponent :type "PrimitiveComponent Object Reference") (OtherActor :type "Actor Object Reference") (OtherComp :type "PrimitiveComponent Object Reference") (OtherBodyIndex :type Integer) (bFromSweep :type Boolean) (SweepResult :type "HitResult Structure (by ref)"))
  (bind _asbp_base_obstacles (cast `/Game/Penjelajah_Spasi/Enemy/Parents/BP_BaseObstacles` OtherActor))
  (set `self.DMG` (`KismetMathLibrary.Conv_IntToDouble` (`/Game/Penjelajah_Spasi/Enemy/Parents/BP_BaseObstacles.HP` _asbp_base_obstacles))))

(fn `UserConstructionScript`
  (`parent.UserConstructionScript`))