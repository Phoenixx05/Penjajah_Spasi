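; Game instance Blueprint that loads and saves the player's high score in a single save slot.
; LoadGame reads HighScore from an SG_SaveGame object if the slot exists, otherwise it prints a notice.
; SaveGame always writes a fresh SG_SaveGame, copying Score into it only when that beats HighScore, so a lower score overwrites the stored record with the class default.
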(event `Load Game`
  (bind _returnvalue (`GameplayStatics.DoesSaveGameExist` "savegame"))
  (if _returnvalue
    (bind _returnvalue_2 (`GameplayStatics.LoadGameFromSlot` "savegame"))
    (bind _assg_save_game (cast `/Game/Penjelajah_Spasi/SG_SaveGame` _returnvalue_2))
    (set `self.HighScore` (`/Game/Penjelajah_Spasi/SG_SaveGame.HighScore` _assg_save_game))
    (else
      (`KismetSystemLibrary.PrintString` "Save game doesn't exist"))))

(event `SaveGame`
  (bind _score (`self.Score`))
  (`KismetSystemLibrary.PrintString` "SAVE")
  (bind _returnvalue (`GameplayStatics.CreateSaveGameObject` "/Game/Penjelajah_Spasi/SG_SaveGame.SG_SaveGame_C"))
  (if (> _score (`self.HighScore`))
    (set `/Game/Penjelajah_Spasi/SG_SaveGame.HighScore` _score _returnvalue))
  (`GameplayStatics.SaveGameToSlot` _returnvalue "savegame"))