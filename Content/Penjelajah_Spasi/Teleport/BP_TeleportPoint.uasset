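; BP_TeleportPoint is a black hole portal that moves the player ship (BP_Pesawat) between the normal map and the boss map.
; On BeginPlay it infers its side by comparing the black hole's location to a hardcoded position.
; On overlap from the normal side, it teleports the ship, spawns BP_MapBoss and clears BP_SpawnMap's child chunks and enemies.
; From the boss side, it teleports back and spawns a new BP_SpawnMap; either way it destroys itself.
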(event `self.ReceiveBeginPlay`
  ;[1 1 1] Cari Tahu Posisi Teleport dan Posisi Pesawat
  (set `self.NotInMapBoss?` (not (== (`SceneComponent.K2_GetComponentLocation` (`self.BlackHole`)) (-15070.931099 -1741.280743 26739.018325)))))

(event `self.Box.OnComponentBeginOverlap`
  (params (OverlappedComponent :type "PrimitiveComponent Object Reference") (OtherActor :type "Actor Object Reference") (OtherComp :type "PrimitiveComponent Object Reference") (OtherBodyIndex :type Integer) (bFromSweep :type Boolean) (SweepResult :type "HitResult Structure (by ref)"))
  (bind _teleportlocation_location (`KismetMathLibrary.BreakTransform` (`self.TeleportLocation`)))
  (bind _teleportlocationback_location (`KismetMathLibrary.BreakTransform` (`self.TeleportLocationBack`)))
  ;[1 1 1] Teleport
  (bind _asbp_pesawat (cast `/Game/Penjelajah_Spasi/Playable/BP_Pesawat` OtherActor))
  (if (`self.NotInMapBoss?`)
    ;;[0.6453 1 0.5885] Teleport ke Map Boss
    (`SceneComponent.K2_SetWorldTransform` (`Actor.RootComponent` _asbp_pesawat) (`KismetMathLibrary.MakeTransform` _teleportlocation_location) false false)
    (`|SpawnActorFromClass` "/Game/Penjelajah_Spasi/Map/BP_MapBoss.BP_MapBoss_C" (`KismetMathLibrary.MakeTransform` (-19720.0 -2030.0 24230.0)) "Undefined" "MultiplyWithRoot" null null)
    (bind _returnvalue (`GameplayStatics.GetActorOfClass` "/Game/Penjelajah_Spasi/Map/BP_SpawnMap.BP_SpawnMap_C"))
    (set `self.SpawnMap` _returnvalue)
    (for _ (range 11)
      (bind _childactor (`/Game/Penjelajah_Spasi/Map/BP_SpawnMap.ChildActor` _returnvalue))
      (bind _output (`|GetArrayItem` _childactor))
      (`/Engine/EditorBlueprintResources/StandardMacros.IsValid` _output
        (:`Is Valid`
          (for _array_element (`/Game/Penjelajah_Spasi/Map/BP_MapBase.Enemy` _output)
            (`/Engine/EditorBlueprintResources/StandardMacros.IsValid` _array_element
              (:`Is Valid`
                (`self.K2_DestroyActor` _array_element))))
          (`self.K2_DestroyActor` _output)
          (`KismetArrayLibrary.Array_Remove` _childactor))))
    (set `self.DoneTeleportToBoss` true)
    (`KismetSystemLibrary.Delay` 0.2)
    (`self.K2_DestroyActor`)
    (else
      ;;[1 0.855 0.4661] Teleport Kembali ke Map Biasa
      (`SceneComponent.K2_SetWorldTransform` (`Actor.RootComponent` _asbp_pesawat) (`KismetMathLibrary.MakeTransform` _teleportlocationback_location) false false)
      (`|SpawnActorFromClass` "/Game/Penjelajah_Spasi/Map/BP_SpawnMap.BP_SpawnMap_C" (`KismetMathLibrary.MakeTransform` (-11820.0 -5170.0 1960.0)) "Undefined" "MultiplyWithRoot" null null)
      (`self.K2_DestroyActor`))))

(fn `UserConstructionScript`)